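; Player-driven tank pawn with hard-coded keys: W/S drive, A/D turn and SpaceBar fires.
; Each movement key opens and closes a Gate that Tick feeds through a Sequence while held.
; Open gates add forward or backward input to FloatingPawnMovement or apply a fixed per-frame local rotation, so turn speed depends on frame rate.
; Firing spawns a TankShell at the tank's own transform, ignoring collisions.
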(event `Key|W`
  (params (Key :type "Key Structure"))
  (:`Pressed`
    (goto _label :!via `Open`))
  (:`Released`
    (goto _label :!via `Close`)))

(event `Key|S`
  (params (Key :type "Key Structure"))
  (:`Pressed`
    (goto _label_2 :!via `Open`))
  (:`Released`
    (goto _label_2 :!via `Close`)))

(event `self.ReceiveTick`
  (params (DeltaSeconds :type "Float (single-precision)"))
  (bind _returnvalue (`self.GetActorForwardVector`))
  (bind _floatingpawnmovement (`self.FloatingPawnMovement`))
  (`|ExecutionSequence`
    (:`then_0`
      (`/Engine/EditorBlueprintResources/StandardMacros.Gate` true :!label _label
        (:`Exit`
          (`PawnMovementComponent.AddInputVector` _floatingpawnmovement _returnvalue false))))
    (:`then_1`
      (`/Engine/EditorBlueprintResources/StandardMacros.Gate` true :!label _label_2
        (:`Exit`
          (`PawnMovementComponent.AddInputVector` _floatingpawnmovement (* _returnvalue (-1.0 -1.0 -1.0)) false))))
    (:`then_2`
      (`/Engine/EditorBlueprintResources/StandardMacros.Gate` true :!label _label_3
        (:`Exit`
          (`self.K2_AddActorLocalRotation` (struct :`Yaw` -1.0)))))
    (:`then_3`
      (`/Engine/EditorBlueprintResources/StandardMacros.Gate` true :!label _label_4
        (:`Exit`
          (`self.K2_AddActorLocalRotation` (struct :`Yaw` 1.0)))))))

(event `Key|A`
  (params (Key :type "Key Structure"))
  (:`Pressed`
    (goto _label_3 :!via `Open`))
  (:`Released`
    (goto _label_3 :!via `Close`)))

(event `Key|D`
  (params (Key :type "Key Structure"))
  (:`Pressed`
    (goto _label_4 :!via `Open`))
  (:`Released`
    (goto _label_4 :!via `Close`)))

(event `Key|SpaceBar`
  (params (Key :type "Key Structure"))
  (:`Pressed`
    (`|SpawnActorFromClass` "/Game/Blueprints/TankShell.TankShell_C" (`self.GetTransform`) "AlwaysSpawn" "MultiplyWithRoot" null null)))

(fn `UserConstructionScript`)