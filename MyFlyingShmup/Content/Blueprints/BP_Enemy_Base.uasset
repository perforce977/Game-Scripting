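; BP_Enemy_Base is an enemy base actor with health, a widget health bar, and death handling.
; Incoming damage lowers Health and updates the bar; surviving hits play a sound and briefly flash an overlay material on all static meshes.
; At zero health it plays an explosion sound, shakes the player's camera, spawns an actor in place and destroys itself.
; Overlapping actors receive damage equal to the enemy's MaxHealth.
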(event `self.ReceiveBeginPlay`
  ; Always Begin with Max Health
  (set `self.Health` (`self.MaxHealth`)))

(event `self.ReceiveAnyDamage`
  (params (Damage :type "Float (single-precision)") (DamageType :type "DamageType Object Reference") (InstigatedBy :type "Controller Object Reference") (DamageCauser :type "Actor Object Reference"))
  (`self.ApplyDamage` Damage)
  ; If Health 0, Begin Death Sequence
  (if (<= (`self.Health`) 0.0)
    (`GameplayStatics.PlaySound2D` "/Game/StarterContent/Audio/Explosion01.Explosion01" 1.0 1.0 0.0 null null)
    ; Death Sequence
    (`|ExecutionSequence`
      (:`then_0`
        (bind _asmy_player_controller (cast `/Game/Framework/myPlayerController` (`GameplayStatics.GetPlayerController` 0)))
        (`/Game/Framework/myPlayerController.ApplyCameraShake` _asmy_player_controller))
      (:`then_1`
        (`|SpawnActorFromClass` "/Game/Particles/BP_Enemy_DeathExplosion.BP_Enemy_DeathExplosion_C" (`KismetMathLibrary.MakeTransform` (`self.K2_GetActorLocation`)) "AlwaysSpawn" "MultiplyWithRoot" null null))
      (:`then_2`
        (`self.K2_DestroyActor`)))
    (else
      (`GameplayStatics.PlaySound2D` "/Game/Audio/Hit.Hit" 1.0 1.0 0.0 null null)
      ; Make M_DamageFlash Instance for BP_Enemy_A
      (for _array_element (`self.K2_GetComponentsByClass` "/Script/Engine.StaticMeshComponent")
        (`MeshComponent.SetOverlayMaterial` _array_element "/Game/Materials/M_DamageFlash.M_DamageFlash"))
      (`KismetSystemLibrary.Delay` 0.2)
      (for _array_element_2 (`self.K2_GetComponentsByClass` "/Script/Engine.StaticMeshComponent")
        (`MeshComponent.SetOverlayMaterial` _array_element_2 null)))))

(event `self.ReceiveActorBeginOverlap`
  (params (OtherActor :type "Actor Object Reference"))
  ; Overlap Damage
  (`GameplayStatics.ApplyDamage` OtherActor (`self.MaxHealth`)))

(event `ApplyDamage`
  (params (Damage :type "Float (double-precision)"))
  ; Damage To Health
  (set `self.Health` (- (`self.Health`) Damage))
  ; Set Progress Bar of Widget
  (bind _aswbp_enemy_health_bar (cast `/Game/UI/WBP_EnemyHealthBar` (`WidgetComponent.GetUserWidgetObject` (`self.Widget`))))
  (`/Game/UI/WBP_EnemyHealthBar.SetHealth` _aswbp_enemy_health_bar (/ (`self.Health`) (`self.MaxHealth`))))

(fn `UserConstructionScript`)