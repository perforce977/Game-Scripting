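; BP_Enemy_Turret is an enemy turret that tracks the player and fires bullets at a steady interval.
; On BeginPlay it starts a looping timer that spawns a BP_Enemy_Bullet at the TurretCapsule's world transform, always spawning regardless of collision.
; Each Tick it turns TurretCapsule toward player pawn 0 using only the look-at yaw, so shots leave along a level heading.
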(event `self.ReceiveBeginPlay`
  (`parent.ReceiveBeginPlay`)
  (`KismetSystemLibrary.K2_SetTimerDelegate` (delegate `ShootBullet`) 2.5 true))

(event `ShootBullet`
  (`|SpawnActorFromClass` "/Game/Blueprints/BP_Enemy_Bullet.BP_Enemy_Bullet_C" (`SceneComponent.K2_GetComponentToWorld` (`self.Turret_Capsule`)) "AlwaysSpawn" "MultiplyWithRoot" null null))

(event `self.ReceiveTick`
  (params (DeltaSeconds :type "Float (single-precision)"))
  (bind (_returnvalue_roll _returnvalue_pitch _returnvalue_yaw) (`KismetMathLibrary.BreakRotator` (`KismetMathLibrary.FindLookAtRotation` (`self.K2_GetActorLocation`) (`self.K2_GetActorLocation` (`GameplayStatics.GetPlayerPawn` 0)))))
  (`SceneComponent.K2_SetWorldRotation` (`self.Turret_Capsule`) (`KismetMathLibrary.MakeRotator` 0.0 0.0 _returnvalue_yaw) false false))

(fn `UserConstructionScript`
  (`parent.UserConstructionScript`))