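; Boss enemy Blueprint that scripts the first boss's entrance and lateral movement, extending a parent class.
; On BeginPlay a timeline slides it along the X axis from its spawn location into the play area.
; When that finishes, it re-captures its location and a slowed second timeline drives side-to-side Y movement from that point.
; Both moves use swept location updates; Tick is empty and the overlap handler is disabled.
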(event `self.ReceiveBeginPlay`
  (`parent.ReceiveBeginPlay`)
  (`self.EnterPlayArea`))

(event `EnterPlayArea`
  (set `self.InitialLocation` (`self.K2_GetActorLocation`))
  (bind (_direction _x_offset) (`Timeline|TL_EnterPlayArea` :!via `PlayFromStart`)
    (:`Update`
      (`self.K2_SetActorLocation` (+ (`self.InitialLocation`) (`KismetMathLibrary.MakeVector` (* _x_offset -2000.0))) true))
    (:`Finished`
      (`self.MoveSidetoSide`))))

(event `MoveSidetoSide`
  (set `self.InitialLocation` (`self.K2_GetActorLocation`))
  (`TimelineComponent.SetPlayRate` (`self.TL_MoveSidetoSide`) 0.2)
  (bind (_direction _y_value) (`Timeline|TL_MoveSidetoSide`)
    (:`Update`
      (`self.K2_SetActorLocation` (+ (`self.InitialLocation`) (`KismetMathLibrary.MakeVector` 0.0 (* _y_value 1500.0))) true))))

(fn `UserConstructionScript`
  (`parent.UserConstructionScript`))